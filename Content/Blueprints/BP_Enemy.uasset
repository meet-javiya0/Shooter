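; Enemy character that chases the player, attacks in melee, takes damage and dies.
; Entering its detection sphere starts a self-repeating AI MoveTo toward the player.
; A one-second loop from BeginPlay plays an attack montage and applies delayed damage while the player is in the attack radius.
; At zero health it ragdolls and is destroyed after a delay; Tick turns and updates its widget health bar.
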(event OnComponentBeginOverlap(Detect_Radius)
  (params (OverlappedComponent :type Primitive%20Component%20Object%20Reference) (OtherActor :type Actor%20Object%20Reference) (OtherComp :type Primitive%20Component%20Object%20Reference) (OtherBodyIndex :type Integer) (bFromSweep :type Boolean) (SweepResult :type Hit%20Result%20Structure%20%28by%20ref%29))
  ;[0.05098 0.05098 0.05098] Chase Player System
  (Utilities|Casting|CastToBP_ThirdPersonCharacter OtherActor)
  (CallFunction|ChasePlayer))

(event OnComponentBeginOverlap(Attack_Raidus)
  (params (OverlappedComponent :type Primitive%20Component%20Object%20Reference) (OtherActor :type Actor%20Object%20Reference) (OtherComp :type Primitive%20Component%20Object%20Reference) (OtherBodyIndex :type Integer) (bFromSweep :type Boolean) (SweepResult :type Hit%20Result%20Structure%20%28by%20ref%29))
  ;[0.05098 0.05098 0.05098] Attack Player System
  (Utilities|Casting|CastToBP_ThirdPersonCharacter OtherActor)
  (Variables|Default|SetIsInRadius true))

(event OnComponentEndOverlap(Attack_Raidus)
  (params (OverlappedComponent :type Primitive%20Component%20Object%20Reference) (OtherActor :type Actor%20Object%20Reference) (OtherComp :type Primitive%20Component%20Object%20Reference) (OtherBodyIndex :type Integer))
  ;[0.05098 0.05098 0.05098] Attack Player System
  (Utilities|Casting|CastToBP_ThirdPersonCharacter OtherActor)
  (Variables|Default|SetIsInRadius false))

(event Custom|Chase%20Player
  ;[0.05098 0.05098 0.05098] Chase Player System
  (if (not (Variables|Default|GetIsEnemyDied))
    (AI|AIMoveTo self "0, 0, 0" (Game|GetPlayerCharacter 0) 1.2e+02 false
      (:OnSuccess
        (CallFunction|ChasePlayer)))))

(event Custom|Attack%20Player
  ;[0.05098 0.05098 0.05098] Attack Player System
  (if (not (Variables|Default|GetIsEnemyDied))
    (if (Variables|Default|GetIsInRadius)
      (Animation|PlayAnimMontage "/Game/EnemyAnimations/Enemy_Attack_Montage.Enemy_Attack_Montage" 1.0 "None")
      (Utilities|FlowControl|Delay 0.25)
      (Utilities|Casting|CastToBP_ThirdPersonCharacter (Game|GetPlayerCharacter 0))
      (Game|Damage|ApplyDamage (Game|GetPlayerCharacter 0) 1e+01 0 0)
      (Development|PrintString "10 Damage to Player"))))

(event EventTick
  (params (DeltaSeconds :type Float%20%28single-precision%29))
  ;[0.05098 0.05098 0.05098] Enemy Healthbar
  (Transformation|SetWorldRotation (Variables|Default|GetHealthbar) (Math|Rotator|FindLookatRotation (Transformation|GetWorldLocation (Variables|Default|GetHealthbar)) (Transformation|GetActorLocation (Game|GetPlayerCharacter 0))) false false)
  (bind _aswb_enemy_healthbar (Utilities|Casting|CastToWB_EnemyHealthbar (UserInterface|GetWidget (Variables|Default|GetHealthbar))))
  (Progress|SetPercent (Variables|/Game/UI/WB_EnemyHealthbar.WB_EnemyHealthbar_C|GetHealthbar_Enemy _aswb_enemy_healthbar) (/ (Variables|Default|GetHealth) 1e+02)))

(event Game|Damage|EventAnyDamage
  (params (Damage :type Float%20%28single-precision%29) (DamageType :type Damage%20Type%20Object%20Reference) (InstigatedBy :type Controller%20Object%20Reference) (DamageCauser :type Actor%20Object%20Reference))
  ;[0.05098 0.05098 0.05098] Health System
  (Variables|Default|SetHealth (- (Variables|Default|GetHealth) Damage))
  (if (not (Variables|Default|GetIsEnemyDied))
    (Niagara|SpawnSystematLocation "/Game/NiagaraSystems/NS_Damage.NS_Damage" (Transformation|GetActorLocation) "0, 0, 0" "1.000000,1.000000,1.000000" true true "AutoRelease")
    (if (<= (Variables|Default|GetHealth) 0.0)
      (Physics|SetSimulatePhysics (Variables|Character|GetMesh) true)
      (Components|Movement|StopMovementImmediately (Variables|Character|GetCharacterMovement))
      (Variables|Default|SetIsEnemyDied true)
      (Utilities|FlowControl|Delay 5.0)
      (Actor|DestroyActor))))

(event EventBeginPlay
  ;[0.05098 0.05098 0.05098] Attack Player System
  (Utilities|FlowControl|RetriggerableDelay 1.0 :!label _label)
  (CallFunction|AttackPlayer)
  (goto _label))

(fn ConstructionScript)